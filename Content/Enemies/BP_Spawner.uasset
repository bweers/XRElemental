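; Enemy spawner that keeps spawning on a looping timer until the level's BP_Enemy count reaches a set maximum.
; Each tick of the timer recounts enemies, then spawns at a random point inside the SpawnArea box if under the cap.
; Spawning requires a valid VRPawn, looked up at BeginPlay and passed as Instigator.
; A separate DestroyAllEnemies event destroys every BP_Enemy in the level.
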(event Custom|SpawnEnemy
  (bind _spawn_area (Variables|Default|GetSpawn%20Area))
  (bind _outactors (Actor|GetAllActorsOfClass "/Game/Enemies/BP_Enemy.BP_Enemy_C"))
  (if (>= (Utilities|Array|Length _outactors) (Variables|Default|GetMaxNumberOfEnemies))
    (Variables|Default|SetMaxEnemiesReached true)
    (else
      (Variables|Default|SetMaxEnemiesReached false)
      (if (not (Variables|Default|GetMaxEnemiesReached))
        (Utilities|IsValid (Utilities|Array|Get(acopy) (stale EventBeginPlay _outactors))
          (:Is%20Valid
            (Game|SpawnActorfromClass "/Game/Enemies/BP_Enemy.BP_Enemy_C" (Math|Transform|MakeTransform (Math|Random|RandomPointinBoundingBox (Transformation|GetWorldLocation _spawn_area) (Components|Box|GetScaledBoxExtent _spawn_area))) "Undefined" 0 (Utilities|Array|Get(acopy) (stale EventBeginPlay _outactors)))))))))

(event Custom|DestroyAllEnemies
  ;[1 1 1] Destroy all Enemies
  (Development|PrintString "Destroy All Enemies Called")
  (bind _outactors (Actor|GetAllActorsOfClass "/Game/Enemies/BP_Enemy.BP_Enemy_C"))
  (for _array_element _outactors
    (Actor|DestroyActor _array_element)))

(event EventBeginPlay
  (Utilities|Time|SetTimerbyEvent (delegate Custom|SpawnEnemy) (Variables|Default|GetSpawnInterval) true 1.0)
  (bind _outactors (Actor|GetAllActorsOfClass "/Game/Blueprints/BaseGame/Player/VRPawn.VRPawn_C"))
  (Input|EnableInput 0))

(event Collision|EventActorBeginOverlap
  (params (OtherActor :type Actor%20Object%20Reference)))

(event EventTick
  (params (DeltaSeconds :type Float%20%28single-precision%29)))

(fn ConstructionScript)